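; BP_BasicEnemy is a basic patrolling enemy that kills an NNCharacter overlapping its capsule and launches one that hits its head collider upward.
; Each tick it moves along a stored forward vector, which CheckWalls reverses when a short forward trace, ignoring Main actors, hits something.
; A two-second timer re-enables the wall check after each reversal.
; The head hit does not destroy the enemy, as DestroyActor is unconnected.
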(event OnComponentHit(HeadCollider)
  (params (HitComponent :type Primitive%20Component%20Object%20Reference) (OtherActor :type Actor%20Object%20Reference) (OtherComp :type Primitive%20Component%20Object%20Reference) (NormalImpulse :type Vector :default "0, 0, 0") (Hit :type Hit%20Result%20Structure%20%28by%20ref%29))
  (bind _asnncharacter (Utilities|Casting|CastToNNCharacter OtherActor))
  (Character|LaunchCharacter _asnncharacter (* (Math|Vector|Normalize (Math|Vector|GetUpVector (Variables|/Script/Engine.Character|GetCapsuleComponent _asnncharacter))) 7.5e+02) false true))

(event OnComponentBeginOverlap(CapsuleComponent)
  (params (OverlappedComponent :type Primitive%20Component%20Object%20Reference) (OtherActor :type Actor%20Object%20Reference) (OtherComp :type Primitive%20Component%20Object%20Reference) (OtherBodyIndex :type Integer) (bFromSweep :type Boolean) (SweepResult :type Hit%20Result%20Structure%20%28by%20ref%29))
  (bind _asnncharacter (Utilities|Casting|CastToNNCharacter OtherActor))
  (Default|Die _asnncharacter))

(event Custom|CheckActive
  (Variables|Default|SetCanCheckWall true)
  (Utilities|Time|ClearandInvalidateTimerbyHandle (stale EventTick _returnvalue)))

(event EventBeginPlay
  (Variables|Default|Setforward (Transformation|GetActorForwardVector)))

(event EventTick
  (params (DeltaSeconds :type Float%20%28single-precision%29))
  (if true
    (Pawn|Input|AddMovementInput (Variables|Default|Getforward) (Variables|Default|Getdirection) false)
    (bind _walldetected (CallFunction|CheckWalls))
    (if _walldetected
      (bind _returnvalue (Utilities|Time|SetTimerbyEvent (delegate Custom|CheckActive) 2.0)))))

(fn ConstructionScript)

(fn CheckWalls
  (bind _returnvalue (Transformation|GetActorLocation))
  (if (Variables|Default|GetCanCheckWall)
    (bind _outactors (Actor|GetAllActorsOfClass "/Game/Characters/Main/Main.Main_C"))
    (bind _returnvalue_2 (Collision|LineTraceByChannel _returnvalue (+ _returnvalue (* (Math|Vector|Normalize (Transformation|GetActorForwardVector)) 25.0)) "TraceTypeQuery1" false _outactors "None"))
    (if _returnvalue_2
      (Variables|Default|Setforward (* (Variables|Default|Getforward) -1.0))
      (Variables|Default|SetCanCheckWall false))
    (return _returnvalue_2)
    (else
      (return false))))